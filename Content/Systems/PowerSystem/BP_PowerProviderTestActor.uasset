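; Test actor for the power system that wraps a PowerProviderComponent and logs its enabled state on BeginPlay.
; A received trigger calls ServerTogglePowerProvider, which flips the provider between enabled and disabled only with authority and logs the result.
; Connect registers the provider component as a member of a given connection point, if that point is valid.
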(event `self.ReceiveBeginPlay`
  (`KismetSystemLibrary.LogString` (`KismetTextLibrary.Conv_TextToString` (`|FormatText` "Provider is {status}" (`KismetMathLibrary.SelectString` "Enabled" "Disabled" (`PowerCircuitMember.GetIsEnabled` (`self.PowerProviderComponent`)))))))

(event `ServerTogglePowerProvider`
  (bind _powerprovidercomponent (`self.PowerProviderComponent`))
  (`/Engine/EditorBlueprintResources/ActorMacros.Switch Has Authority`
    (:`Authority`
      (if (`PowerCircuitMember.GetIsEnabled` (`self.PowerProviderComponent`))
        (`PowerCircuitMember.Disable` _powerprovidercomponent)
        (`KismetSystemLibrary.LogString` "Disabled provider")
        (else
          (`PowerCircuitMember.Enable` _powerprovidercomponent)
          (`KismetSystemLibrary.LogString` "Enabled provider"))))))

(event `TriggerReceiverInterface.OnTriggerReceived`
  (params (TriggerPayload :type "Object Object Reference"))
  (`self.ServerTogglePowerProvider`))

(fn `Connect`
  (params (ConnectionPoint :type "PowerCircuitConnectionPointComponent Object Reference"))
  (`/Engine/EditorBlueprintResources/StandardMacros.IsValid` ConnectionPoint
    (:`Is Valid`
      (`PowerCircuitConnectionPointComponent.ConnectMember` ConnectionPoint (`self.PowerProviderComponent`)))))

(fn `UserConstructionScript`)