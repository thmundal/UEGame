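; Test actor for the power system that displays and logs the state of its power circuit component.
; On BeginPlay and whenever the circuit's power balance changes, it computes the spare capacity fraction, falling back to zero without valid capacity.
; That fraction feeds the PowerStatus bar in an in-world HUD widget.
; Each update also logs capacity and demand, labelled Server on a dedicated server and Client otherwise.
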(event `self.ReceiveBeginPlay`
  (bind _powercircuitcomponent (`self.PowerCircuitComponent`))
  (`self.SetPowerUIPercent` (`self.GetPowerPercent`))
  (`KismetSystemLibrary.LogString` (`KismetTextLibrary.Conv_TextToString` (`|FormatText` "{role} Power changed. Capacity: {capacity} Demand: {demand}" (`KismetMathLibrary.SelectString` "Server" "Client" (`KismetSystemLibrary.IsDedicatedServer`)) (`PowerCircuitComponent.GetPowerCapacity` _powercircuitcomponent) (`PowerCircuitComponent.GetPowerDemand` _powercircuitcomponent))) :!label _label))

(event `self.PowerCircuitComponent.m_OnPowerBalanceChanged`
  (`self.SetPowerUIPercent` (`self.GetPowerPercent`))
  (goto _label))

(fn `GetPowerPercent`
  (returns (Percent :type "Float (double-precision)"))
  (bind _powercircuitcomponent (`self.PowerCircuitComponent`)
    (:`then`
      (bind _returnvalue (`PowerCircuitComponent.GetPowerCapacity` _powercircuitcomponent))
      (if (> _returnvalue 0.0)
        (return (- 1.0 (/ (`PowerCircuitComponent.GetPowerDemand` _powercircuitcomponent) _returnvalue)))
        (else
          _)))
    (:`else`
      _))
  (return 0.0))

(fn `GetPowerStatusWidget`
  (returns (PowerStatus :type "ProgressBar Object Reference"))
  (bind _asw_power_provider_in_world_hud (cast `/Game/Systems/PowerSystem/Widgets/W_PowerProviderInWorldHud` (`WidgetComponent.GetWidget` (`self.PowerBarWidget`))))
  (return (`/Game/Systems/PowerSystem/Widgets/W_PowerProviderInWorldHud.PowerStatus` _asw_power_provider_in_world_hud)))

(fn `SetPowerUIPercent`
  (params (InPercent :type "Float (single-precision)"))
  (bind _powerstatus (`self.GetPowerStatusWidget`))
  (`/Engine/EditorBlueprintResources/StandardMacros.IsValid` _powerstatus
    (:`Is Valid`
      (`ProgressBar.SetPercent` _powerstatus InPercent))))

(fn `UserConstructionScript`)