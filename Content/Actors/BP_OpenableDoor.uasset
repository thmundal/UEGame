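; BP_OpenableDoor is a door actor that slides along its local Z axis between its starting position and a maximum offset.
; OnTriggerReceived toggles the Open flag, which sets the direction of travel.
; Tick moves the whole actor by a step scaled by delta time, accumulates the current offset, and stops moving once it reaches or passes either limit, without clamping.
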(event `self.ReceiveTick`
  (params (DeltaSeconds :type "Float (single-precision)"))
  (bind _currentzoffset (`self.CurrentZOffset`))
  (bind _returnvalue (* (`self.OffsetStep`) (`KismetMathLibrary.SelectInt` 1 -1 (`self.Open`))))
  (bind _returnvalue_2 (* (`KismetMathLibrary.SelectFloat` (`KismetMathLibrary.SelectFloat` 0.0 _returnvalue (>= _currentzoffset (`self.MaxZOffset`))) (`KismetMathLibrary.SelectFloat` 0.0 _returnvalue (<= _currentzoffset 0.0)) (`self.Open`)) (`GameplayStatics.GetWorldDeltaSeconds`)))
  (`self.K2_AddActorLocalOffset` (`KismetMathLibrary.MakeVector` 0.0 0.0 _returnvalue_2))
  (set `self.CurrentZOffset` (+ (`self.CurrentZOffset`) _returnvalue_2)))

(event `TriggerReceiverInterface.OnTriggerReceived`
  (params (TriggerPayload :type "Object Object Reference"))
  (set `self.Open` (not (`self.Open`))))

(fn `UserConstructionScript`)